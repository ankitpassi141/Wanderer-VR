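; Speed boost Blueprint that temporarily raises the player's walk speed through overlap with its SpeedBoost component.
; Begin overlap adds a child actor component to player 0 and sets MaxWalkSpeed to their current velocity magnitude scaled by Boost.
; End overlap waits five seconds, then the FastToSlow timeline lerps the current speed toward OriginalSpeed.
; Both events act on player 0 without checking the overlapping actor.
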(event OnComponentBeginOverlap(SpeedBoost)
  (params (OverlappedComponent :type Primitive%20Component%20Object%20Reference) (OtherActor :type Actor%20Object%20Reference) (OtherComp :type Primitive%20Component%20Object%20Reference) (OtherBodyIndex :type Integer) (bFromSweep :type Boolean) (SweepResult :type Hit%20Result%20Structure%20%28by%20ref%29))
  (bind _returnvalue (Game|GetPlayerCharacter 0))
  (AddComponent|AddChildActorComponent _returnvalue false)
  (bind _output_get (Variables|/Script/Engine.CharacterMovementComponent|SetMaxWalkSpeed (Variables|/Script/Engine.Character|GetCharacterMovement _returnvalue) (Math|Vector|VectorLength (* (Transformation|GetVelocity _returnvalue) (Variables|Default|GetBoost))))))

(event OnComponentEndOverlap(SpeedBoost)
  (params (OverlappedComponent :type Primitive%20Component%20Object%20Reference) (OtherActor :type Actor%20Object%20Reference) (OtherComp :type Primitive%20Component%20Object%20Reference) (OtherBodyIndex :type Integer))
  (Utilities|FlowControl|Delay 5.0)
  (bind _newtrack_0 (Timeline|Fast%20to%20slow Play)
    (:Update
      (Variables|/Script/Engine.CharacterMovementComponent|SetMaxWalkSpeed (Variables|/Script/Engine.Character|GetCharacterMovement (Game|GetPlayerCharacter 0)) (Math|Float|Lerp (stale OnComponentBeginOverlap(SpeedBoost) _output_get) (Variables|Default|GetOriginal_Speed) _newtrack_0)))))

(fn ConstructionScript)